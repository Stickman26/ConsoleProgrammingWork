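; BP_Projectile is a projectile Blueprint with logic for shrinking the actor it strikes, currently left unwired.
; Its Hit event is empty, and a disconnected chain would destroy the projectile, then call ShrinkSize if the hit actor's name string lacks "None".
; ShrinkSize halves the actor's scale, then calls ChangeColor if it is an EditorCube_Blueprint.
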(event Collision|EventHit
  (params (MyComp :type Primitive%20Component%20Object%20Reference) (Other :type Actor%20Object%20Reference) (OtherComp :type Primitive%20Component%20Object%20Reference) (bSelfMoved :type Boolean) (HitLocation :type Vector :default "0, 0, 0") (HitNormal :type Vector :default "0, 0, 0") (NormalImpulse :type Vector :default "0, 0, 0") (Hit :type Hit%20Result%20Structure%20%28by%20ref%29)))

(fn ConstructionScript)

(fn ShrinkSize
  (params (ActorHit :type Actor%20Object%20Reference))
  (bind _output_get (Variables|Default|SetSize (/ (Transformation|GetActorScale3D ActorHit) 2)))
  (Transformation|SetActorScale3D ActorHit _output_get)
  (bind _aseditor_cube_blueprint (Utilities|Casting|CastToEditorCube_Blueprint ActorHit))
  (Default|ChangeColor _aseditor_cube_blueprint)
  (return))